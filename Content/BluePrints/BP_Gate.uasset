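; BP_Gate is a gate Blueprint that dissolves and stops blocking when opened.
; On BeginPlay it creates a dynamic instance of M_Gate on the Cube mesh and stores it.
; The GateOpen event plays a timeline that drives the material's opacity and wall color, then disables the Cube's collision when finished.
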(event Custom|GateOpen
  (bind (_direction _dissolve _color) (Timeline|Timeline Play)
    (:Update
      (Rendering|Material|SetScalarParameterValueonMaterials (Variables|Default|GetCube) "Opacity" _dissolve)
      (Rendering|Material|SetVectorParameterValue (Variables|Default|GetGateColour) "WallColor" _color :!class /Script/Engine.MaterialInstanceDynamic))
    (:Finished
      (Collision|SetCollisionEnabled (Variables|Default|GetCube) "NoCollision"))))

(event EventBeginPlay
  (bind _returnvalue (Rendering|Material|CreateDynamicMaterialInstance (Variables|Default|GetCube) 0 "/Game/Materials/M_Gate.M_Gate" "None" :!class /Script/Engine.PrimitiveComponent))
  (Variables|Default|SetGateColour _returnvalue))

(fn ConstructionScript)