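; BP_ArrowUpDown is an arrow marker that bobs vertically and opens a linked gate when the player touches it.
; On BeginPlay, the UpDown timeline plays and drives the arrow's relative Z location.
; When the player character overlaps the Box, the arrow hides, the box's collision turns off so it fires once, and GateOpen is called on the Gate reference.
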(event OnComponentBeginOverlap(Box)
  (params (OverlappedComponent :type Primitive%20Component%20Object%20Reference) (OtherActor :type Actor%20Object%20Reference) (OtherComp :type Primitive%20Component%20Object%20Reference) (OtherBodyIndex :type Integer) (bFromSweep :type Boolean) (SweepResult :type Hit%20Result%20Structure%20%28by%20ref%29))
  (if (== OtherActor (Game|GetPlayerCharacter 0))
    (Rendering|SetVisibility (Variables|Default|GetArrow) false false)
    (Collision|SetCollisionEnabled (Variables|Default|GetBox) "NoCollision")
    (Default|GateOpen (Variables|Default|GetGate))))

(event Custom|UpDownEvent
  (bind _movement (Timeline|UpDown Play)
    (:Update
      (Transformation|SetRelativeLocation (Variables|Default|GetArrow) (Math|Vector|MakeVector 0.0 0.0 _movement) false false))))

(event EventBeginPlay
  (CallFunction|UpDownEvent))

(fn ConstructionScript)