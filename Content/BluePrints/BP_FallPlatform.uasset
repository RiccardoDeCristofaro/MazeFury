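; BP_FallPlatform is a platform that reacts to the player character by changing color or falling.
; BeginPlay creates a dynamic instance of M_Fluo on the static mesh.
; On player overlap, a timeline drives the material's Color parameter, or, if Fallen is already true, the mesh starts simulating physics.
; The graph only reads Fallen and never sets it.
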(event OnComponentBeginOverlap(StaticMesh)
  (params (OverlappedComponent :type Primitive%20Component%20Object%20Reference) (OtherActor :type Actor%20Object%20Reference) (OtherComp :type Primitive%20Component%20Object%20Reference) (OtherBodyIndex :type Integer) (bFromSweep :type Boolean) (SweepResult :type Hit%20Result%20Structure%20%28by%20ref%29))
  (if (== OtherActor (Game|GetPlayerCharacter 0))
    (if (Variables|Default|GetFallen)
      (Physics|SetSimulatePhysics (Variables|Default|GetStaticMesh) true)
      (else
        (bind _newcolor (Timeline|Timeline Play)
          (:Update
            (Rendering|Material|SetVectorParameterValue (stale EventBeginPlay _returnvalue) "Color" _newcolor :!class /Script/Engine.MaterialInstanceDynamic)))))))

(event EventBeginPlay
  (bind _returnvalue (Rendering|Material|CreateDynamicMaterialInstance (Variables|Default|GetStaticMesh) 0 "/Game/Materials/M_Fluo.M_Fluo" "None" :!class /Script/Engine.PrimitiveComponent)))

(fn ConstructionScript)