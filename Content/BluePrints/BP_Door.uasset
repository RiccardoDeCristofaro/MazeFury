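; Door Blueprint that slides open when the player character enters its trigger Box while ShouldOpen is true.
; The OpenDoor timeline moves the Cube along local Z through a track named Rotation, holding Y fixed.
; Leaving the Box reverses the timeline without checking ShouldOpen.
; The timeline's Finished output calls GateOpen on the Gate reference, which also fires when a reverse completes.
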(event OnComponentBeginOverlap(Box)
  (params (OverlappedComponent :type Primitive%20Component%20Object%20Reference) (OtherActor :type Actor%20Object%20Reference) (OtherComp :type Primitive%20Component%20Object%20Reference) (OtherBodyIndex :type Integer) (bFromSweep :type Boolean) (SweepResult :type Hit%20Result%20Structure%20%28by%20ref%29))
  (if (and (== OtherActor (Game|GetPlayerCharacter 0)) (Variables|Default|GetShouldOpen))
    (bind _rotation (Timeline|OpenDoor Play)
      (:Update
        (Transformation|SetRelativeLocation (Variables|Default|GetCube) (Math|Vector|MakeVector 0.0 -2.9e+02 _rotation) false false))
      (:Finished
        (Default|GateOpen (Variables|Default|GetGate))))))

(event OnComponentEndOverlap(Box)
  (params (OverlappedComponent :type Primitive%20Component%20Object%20Reference) (OtherActor :type Actor%20Object%20Reference) (OtherComp :type Primitive%20Component%20Object%20Reference) (OtherBodyIndex :type Integer))
  (if (== OtherActor (Game|GetPlayerCharacter 0))
    (bind _rotation (Timeline|OpenDoor Reverse)
      (:Update
        (Transformation|SetRelativeLocation (Variables|Default|GetCube) (Math|Vector|MakeVector 0.0 -2.9e+02 _rotation) false false))
      (:Finished
        (Default|GateOpen (Variables|Default|GetGate))))))

(fn ConstructionScript)