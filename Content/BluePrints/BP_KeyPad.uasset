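; BP_KeyPad is an in-world keypad that opens a referenced level door when the correct code is entered.
; On BeginPlay it binds to button clicks from its WBP_KeyPad widget component.
; Each click appends the button index to a combination string shown on a text render.
; The door opens when that string matches the door's combination and is under three characters long; the string is never cleared.
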(event Custom|ButtonClicked
  (params (ButtonIndex :type Integer))
  (bind _output_get (Variables|Default|SetCombination (Utilities|String|Append (Variables|Default|GetCombination) (Utilities|String|ToString(Text) (Utilities|Text|FormatText "{code}" ButtonIndex)))))
  (Rendering|Components|TextRender|SetText (Variables|Default|GetTextRender) (Utilities|Text|ToText(String) _output_get))
  (if (and (Utilities|Enum|Equal(Enum) _output_get (Variables|/Game/BluePrints/BP_level2Door.BP_level2Door_C|GetCombinationDoor (Variables|Default|GetDoorRef))) (< (Utilities|String|Len _output_get) 3))
    (Default|OpenLevelDoor (Variables|Default|GetDoorRef))))

(event EventBeginPlay
  (bind _aswbp_key_pad (Utilities|Casting|CastToWBP_KeyPad (UserInterface|GetWidget (Variables|Default|GetWidget))))
  (EventDispatchers|BindEventtoOnButtonClick _aswbp_key_pad (delegate Custom|ButtonClicked)))

(fn ConstructionScript)