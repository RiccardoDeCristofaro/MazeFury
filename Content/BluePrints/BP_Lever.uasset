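; BP_Lever is an interactable lever that lowers a linked bridge.
; Overlap on its Box enables player input, and pressing E checks that the last overlapping actor is the player character.
; The LeverPush timeline then drives the Cube's relative pitch and calls LowBridge on the Bridge reference when finished.
; Input is never disabled, as no end-overlap handler exists.
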(event OnComponentBeginOverlap(Box)
  (params (OverlappedComponent :type Primitive%20Component%20Object%20Reference) (OtherActor :type Actor%20Object%20Reference) (OtherComp :type Primitive%20Component%20Object%20Reference) (OtherBodyIndex :type Integer) (bFromSweep :type Boolean) (SweepResult :type Hit%20Result%20Structure%20%28by%20ref%29))
  (Input|EnableInput (Game|GetPlayerController 0)))

(event Input|KeyboardEvents|E
  (params (Key :type Key%20Structure :default "None"))
  (:Pressed
    (if (== (stale OnComponentBeginOverlap(Box) OtherActor) (Game|GetPlayerCharacter 0))
      (bind _leveron (Timeline|LeverPush Play)
        (:Update
          (Transformation|SetRelativeRotation (Variables|Default|GetCube) (Math|Rotator|MakeRotator 0.0 _leveron 0.0) false false))
        (:Finished
          (Default|LowBridge (Variables|Default|GetBridge)))))))

(fn ConstructionScript)