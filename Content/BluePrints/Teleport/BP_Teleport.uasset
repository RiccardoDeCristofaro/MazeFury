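; BP_Teleport is a trigger actor that teleports the player character to a target point.
; When the first player's character overlaps its Box, it waits through a short Delay, without rechecking the overlap afterwards.
; It then sets the character's root component to the world location of the SpawnPoint on the referenced TargetPoint, using that SpawnPoint's rotation multiplied by minus one.
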(event OnComponentBeginOverlap(Box)
  (params (OverlappedComponent :type Primitive%20Component%20Object%20Reference) (OtherActor :type Actor%20Object%20Reference) (OtherComp :type Primitive%20Component%20Object%20Reference) (OtherBodyIndex :type Integer) (bFromSweep :type Boolean) (SweepResult :type Hit%20Result%20Structure%20%28by%20ref%29))
  (bind _returnvalue (Game|GetPlayerCharacter 0))
  (bind _targetpoint (Variables|Default|GetTargetPoint))
  (if (== OtherActor _returnvalue)
    (Utilities|FlowControl|Delay 2.0)
    (Transformation|SetWorldLocationAndRotation (Variables|/Script/Engine.Actor|GetRootComponent _returnvalue) (Transformation|GetWorldLocation (Variables|BP_Teleport_C|GetSpawnPoint _targetpoint)) (* (Transformation|GetWorldRotation (Variables|BP_Teleport_C|GetSpawnPoint _targetpoint)) -1.0) false false)))

(event EventBeginPlay)

(event Collision|EventActorBeginOverlap
  (params (OtherActor :type Actor%20Object%20Reference)))

(event EventTick
  (params (DeltaSeconds :type Float%20%28single-precision%29)))

(fn ConstructionScript)