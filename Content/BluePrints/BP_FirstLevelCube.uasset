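; BP_FirstLevelCube is a shootable cube that counts toward opening a gate, apparently in the first level.
; A hit on its Box by a BP_FirstPersonProjectile increments the Manager's cube count, refreshes it through UpdateCubes and destroys the cube.
; When the count reaches the Manager's MaxCubes, it also calls GateOpen on the Gate and sets MaxReached on the Manager.
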(event OnComponentHit(Box)
  (params (HitComponent :type Primitive%20Component%20Object%20Reference) (OtherActor :type Actor%20Object%20Reference) (OtherComp :type Primitive%20Component%20Object%20Reference) (NormalImpulse :type Vector :default "0, 0, 0") (Hit :type Hit%20Result%20Structure%20%28by%20ref%29))
  (Utilities|Casting|CastToBP_FirstPersonProjectile OtherActor)
  (bind _result (Math|Integer|IncrementInt (Variables|/Game/BluePrints/BP_Level1Manager.BP_Level1Manager_C|GetCubes (Variables|Default|GetManager)))
    (:%20%20
      (if (>= _result (Variables|/Game/BluePrints/BP_Level1Manager.BP_Level1Manager_C|GetMaxCubes (Variables|Default|GetManager)))
        (Default|UpdateCubes (Variables|Default|GetManager))
        (Actor|DestroyActor)
        (Default|GateOpen (Variables|Default|GetGate))
        (Variables|/Game/BluePrints/BP_Level1Manager.BP_Level1Manager_C|SetMaxReached (Variables|Default|GetManager) true)
        (else
          (Actor|DestroyActor)
          (Default|UpdateCubes (Variables|Default|GetManager)))))))

(fn ConstructionScript)