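; BP_ky_magicCircle1 is a magic circle effect actor that damages actors standing inside its Box volume.
; Beginning an overlap applies damage to that actor and starts a looping half-second timer that re-runs StartDamaging, which re-sets the timer each time.
; Ending any overlap clears that single timer handle.
; The construction script passes the Color variable to the Fx component's color parameter.
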(event OnComponentBeginOverlap(Box)
  (params (OverlappedComponent :type Primitive%20Component%20Object%20Reference) (OtherActor :type Actor%20Object%20Reference) (OtherComp :type Primitive%20Component%20Object%20Reference) (OtherBodyIndex :type Integer) (bFromSweep :type Boolean) (SweepResult :type Hit%20Result%20Structure%20%28by%20ref%29))
  (CallFunction|StartDamaging))

(event OnComponentEndOverlap(Box)
  (params (OverlappedComponent :type Primitive%20Component%20Object%20Reference) (OtherActor :type Actor%20Object%20Reference) (OtherComp :type Primitive%20Component%20Object%20Reference) (OtherBodyIndex :type Integer))
  (CallFunction|EndDamaging))

(event Custom|EndDamaging
  (Utilities|Time|ClearandInvalidateTimerbyHandle (stale Custom|StartDamaging _returnvalue)))

(event Custom|StartDamaging
  (Game|Damage|ApplyDamage (stale OnComponentBeginOverlap(Box) OtherActor) (Variables|Default|GetDamage) 0 0)
  (bind _returnvalue (Utilities|Time|SetTimerbyEvent (delegate Custom|StartDamaging) 0.5 true)))

(fn ConstructionScript
  (|CallParentFunction)
  (Effects|Components|ParticleSystem|SetVectorParameter (Variables|Default|Getfx) "color" (Math|Conversions|ToVector(LinearColor) (Variables|Default|Getcolor))))